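; BP_monster is a side-scroller monster that patrols along the Y axis using an Idle/Walk/Die state machine run on Tick.
; Idle waits, then picks a random Y target between the walk bounds and prints it for debugging.
; Walk steps a fixed, frame-rate-dependent distance per tick, easing rotation toward the target, and returns to Idle within a speed-derived threshold.
; Die sets a flag and destroys the actor after the death animation delay.
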(event EventTick
  (params (DeltaSeconds :type Float%20%28single-precision%29))
  (bind _returnvalue (Transformation|GetActorLocation))
  (switch Utilities|FlowControl|Switch|SwitchonBPE_Monster_State (Variables|Default|GetCur_State)
    (:NewEnumerator0
      (if (not (Variables|Default|GetDie))
        (Utilities|FlowControl|Delay (Variables|Default|GetWaiting_Time))
        (bind _output_get (Variables|Default|SetTarget_Pos (Math|Vector|MakeVector (.x _returnvalue) (Math|Random|RandomFloatinRange (Variables|Default|GetWalk_Start_Y_Pose) (Variables|Default|GetWalk_End_Y_Pose)) (.z _returnvalue))))
        (Variables|Default|SetCur_State "NewEnumerator1")
        (Development|PrintString (Utilities|String|Append (Utilities|String|ToString(Vector) _output_get) "어디로 가려고 생각함"))))
    (:NewEnumerator1
      (if (not (Variables|Default|GetDie))
        (if (< (Math|Vector|Distance(Vector) (Transformation|GetActorLocation) (Variables|Default|GetTarget_Pos)) (Variables|Default|GetCheck_Close_Target))
          (Variables|Default|SetCur_State "NewEnumerator0")
          (else
            (Transformation|SetActorLocationAndRotation (+ (Transformation|GetActorLocation) (* (Math|Vector|Normalize (Math|Vector|MakeVector 0.0 (.Y (Math|Vector|BreakVector (- (Variables|Default|GetTarget_Pos) (Transformation|GetActorLocation)))) 0.0)) (+ 0.0 (Variables|Default|GetMonster_Speed)))) (Math|Rotator|Lerp(Rotator) (Transformation|GetActorRotation) (Math|Rotator|FindLookatRotation (Transformation|GetActorLocation) (Variables|Default|GetTarget_Pos)) 0.2))))))
    (:NewEnumerator2
      (Variables|Default|SetDie true)
      (Utilities|FlowControl|Delay (Variables|Default|GetDie_Anim_Time))
      (Actor|DestroyActor))))

(fn ConstructionScript
  (Utilities|FlowControl|Sequence
    (:then_0
      (Variables|Default|SetCur_State "NewEnumerator0"))
    (:then_1
      (Variables|Default|SetTarget_Pos (Transformation|GetActorLocation)))
    (:then_2
      (Variables|Default|SetCheck_Close_Target (+ (/ (Variables|Default|GetMonster_Speed) 2.0) 1.0)))))