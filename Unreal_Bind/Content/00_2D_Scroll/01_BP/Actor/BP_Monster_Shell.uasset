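; BP_Monster_Shell is a shell monster for a 2D scroller that hurts the player on contact and reacts to bullets.
; Overlapping man_Character_1 with its Body calls OnLoseHP through a DoOnce that resets immediately, then spawns an explosion at the monster.
; Overlapping a Bullet switches CurState to another enum value and disables Body collision.
; BeginPlay and Tick are empty, and the construction script only calls the parent.
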(event OnComponentBeginOverlap(Body)
  (params (OverlappedComponent :type Primitive%20Component%20Object%20Reference) (OtherActor :type Actor%20Object%20Reference) (OtherComp :type Primitive%20Component%20Object%20Reference) (OtherBodyIndex :type Integer) (bFromSweep :type Boolean) (SweepResult :type Hit%20Result%20Structure%20%28by%20ref%29))
  (Utilities|FlowControl|Sequence
    (:then_0
      (bind _asman_character_1 (Utilities|Casting|CastToman_Character_1 OtherActor))
      (Utilities|FlowControl|Sequence
        (:then_0
          (Utilities|FlowControl|DoOnce false :!label _label
            (:Completed
              (Default|OnLoseHP _asman_character_1))))
        (:then_1
          (goto _label Reset))
        (:then_2
          (Effects|SpawnEmitteratLocation "/Game/00_2D_Scroll/09_Particle/P_Explosion.P_Explosion" (Transformation|GetActorLocation)))))
    (:then_1
      (Utilities|Casting|CastToBullet OtherActor)
      (Variables|Default|SetCur_State "NewEnumerator2")
      (Collision|SetCollisionEnabled (Variables|Default|GetBody) "NoCollision"))))

(event EventBeginPlay)

(event Collision|EventActorBeginOverlap
  (params (OtherActor :type Actor%20Object%20Reference)))

(event EventTick
  (params (DeltaSeconds :type Float%20%28single-precision%29)))

(fn ConstructionScript
  (|CallParentFunction))