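; BP_NPC is a 2D-scroller NPC that shows a dialogue widget while the player character overlaps its Box.
; The construction script loads a fixed data table row into Info, supplying the name and script lines.
; Each overlap creates a UMG_UIE_Dialog on the Widget component and advances ScriptIndex; leaving clears it.
; The modulo-3 selection cycles only the first three of four script lines, so Script3 never appears.
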(event OnComponentBeginOverlap(Box)
  (params (OverlappedComponent :type Primitive%20Component%20Object%20Reference) (OtherActor :type Actor%20Object%20Reference) (OtherComp :type Primitive%20Component%20Object%20Reference) (OtherBodyIndex :type Integer) (bFromSweep :type Boolean) (SweepResult :type Hit%20Result%20Structure%20%28by%20ref%29))
  (bind _info (Variables|Default|GetInfo))
  (bind (_name _script_0 _script_1 _script_2 _script_3) (Utilities|Struct|BreakBPS_NPC_Info _info))
  (Utilities|Casting|CastToman_Character_1 OtherActor)
  (bind _returnvalue (UserInterface|CreateWidget "/Game/00_2D_Scroll/01_BP/UI/UMG_UIE_Dialog.UMG_UIE_Dialog_C" 0 _name (Utilities|Array|Get(acopy) (Utilities|Array|MakeArray _script_0 _script_1 _script_2 _script_3) (Math|Integer|%(Integer) (Variables|Default|GetScript_Index) 3))))
  (UserInterface|SetWidget (Variables|Default|GetWidget) _returnvalue)
  (Variables|Default|SetScript_Index (+ (Variables|Default|GetScript_Index) 1)))

(event OnComponentEndOverlap(Box)
  (params (OverlappedComponent :type Primitive%20Component%20Object%20Reference) (OtherActor :type Actor%20Object%20Reference) (OtherComp :type Primitive%20Component%20Object%20Reference) (OtherBodyIndex :type Integer))
  (Utilities|Casting|CastToman_Character_1 OtherActor)
  (UserInterface|SetWidget (Variables|Default|GetWidget) 0))

(event EventBeginPlay)

(event Collision|EventActorBeginOverlap
  (params (OtherActor :type Actor%20Object%20Reference)))

(event EventTick
  (params (DeltaSeconds :type Float%20%28single-precision%29)))

(fn ConstructionScript
  (bind _returnvalue (Utilities|GetDataTableRow "/Game/00_2D_Scroll/08_Data/수업_-_시트18__1_.수업_-_시트18__1_" "0")
    (:then
      (Variables|Default|SetInfo _returnvalue))))